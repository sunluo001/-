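; Actor that draws a movement path as a line of straight spline mesh segments, with an arrow mesh at the first point.
; DrawMoveLineCustom stores the points raised slightly against Z-fighting, and Tick draws them once, then clears them.
; Segments come from a pool that grows on demand and hides extras.
; SetType recolours the dynamic line and arrow materials for four types, while FadeIn forces full opacity instantly.
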(event Custom|DrawMoveLineCustom
  (params (InputPoints :type Array%20of%20Vectors))
  (bind _output_get (Variables|Default|SetDrawArrPoints InputPoints))
  ;[1 1 1] 抬高10cm,避免渲染贴地Z冲突
  (for (_array_element _array_index) _output_get
    (Utilities|Array|SetArrayElem _output_get _array_index (+ _array_element "0, 0,10.000000")))
  (Variables|Default|SetLastPosNum (Utilities|Array|Length _output_get))
  (CallFunction|Fadein))

(event Custom|SetType
  (params (Selection :type Integer))
  (switch int Selection
    (:0
      (Variables|Default|SetScaleChange false)
      ;[1 1 1] Color0
      (Variables|Default|SetLine&ArrowColor (Utilities|Struct|MakeLinearColor 0.0 1.0 0.0 0.5)))
    (:1
      (Variables|Default|SetScaleChange false)
      ;[1 1 1] Color1
      (Variables|Default|SetLine&ArrowColor (Utilities|Struct|MakeLinearColor 1.0 0.0 0.0 1.0)))
    (:2
      (Variables|Default|SetScaleChange true)
      ;[1 1 1] Color2
      (Variables|Default|SetLine&ArrowColor (Utilities|Struct|MakeLinearColor 35.0 21.0 0.0 1.0)))
    (:3
      (Variables|Default|SetScaleChange true)
      ;[1 1 1] Color3
      (Variables|Default|SetLine&ArrowColor (Utilities|Struct|MakeLinearColor 6.0 0.0 0.0 1.0))))
  (Rendering|Material|SetVectorParameterValue (Variables|Default|GetM_Arrow) "EM_Color" (Variables|Default|GetLine&ArrowColor) :!class /Script/Engine.MaterialInstanceDynamic)
  (Rendering|Material|SetVectorParameterValue (Variables|Default|GetM_Line) "EM_Color" (Variables|Default|GetLine&ArrowColor) :!class /Script/Engine.MaterialInstanceDynamic))

(event EventBeginPlay)

(event Collision|EventActorBeginOverlap
  (params (OtherActor :type Actor%20Object%20Reference)))

(event EventTick
  (params (DeltaSeconds :type Float%20%28single-precision%29))
  (if (> (Variables|Default|GetLastPosNum) 0)
    (CallFunction|DrawMoveLine (Variables|Default|GetDrawArrPoints))
    (Variables|Default|SetLastPosNum 0)
    (Utilities|Array|Clear (Variables|Default|GetDrawArrPoints))))

(fn ConstructionScript
  (bind _returnvalue (Rendering|Material|CreateDynamicMaterialInstance "/Game/Common/Material/MI_Arrow_01_b.MI_Arrow_01_b" "None" "None" :!class /Script/Engine.KismetMaterialLibrary))
  (Variables|Default|SetM_Line _returnvalue)
  (bind _returnvalue_2 (Rendering|Material|CreateDynamicMaterialInstance "/Game/Common/Material/MI_Arrow_01.MI_Arrow_01" "None" "None" :!class /Script/Engine.KismetMaterialLibrary))
  (Variables|Default|SetM_Arrow _returnvalue_2))

(fn DrawMoveLine
  (params (ArrPoint :type Array%20of%20Vectors))
  (CallFunction|ResetSplineMesh ArrPoint)
  (CallFunction|SetSplineMesh ArrPoint)
  (CallFunction|SetArrowMesh ArrPoint))

(fn ResetSplineMesh
  (params (ArrPoints :type Array%20of%20Vectors))
  (LocalVariables|SetNewPosNum (Math|Integer|Max(Integer) (- (Utilities|Array|Length ArrPoints) 1)))
  (LocalVariables|SetOldPosNum (Utilities|Array|Length (Variables|Default|GetSplineMeshPool)))
  (if (> (LocalVariables|GetNewPosNum) (LocalVariables|GetOldPosNum))
    (for _index (range 0 (- (- (LocalVariables|GetNewPosNum) (LocalVariables|GetOldPosNum)) 1))
      (bind _returnvalue (AddComponent|AddSplineMeshComponent false))
      (Rendering|SetRenderCustomDepth _returnvalue false)
      (Components|StaticMesh|SetStaticMesh _returnvalue (Variables|Default|GetLineMesh))
      (Rendering|Material|SetMaterial _returnvalue 0 (Variables|Default|GetM_Line))
      (SplineMesh|SetForwardAxis _returnvalue "X" false)
      (Collision|SetCollisionEnabled _returnvalue "NoCollision")
      (Rendering|SetVisibility _returnvalue false true)
      (Development|SetHiddeninGame _returnvalue true true)
      (if (Variables|Default|GetScaleChange)
        (SplineMesh|SetEndScale _returnvalue "(X=0.200000,Y=0.200000)" true :!class /Script/Engine.SplineMeshComponent)
        (SplineMesh|SetStartScale _returnvalue "(X=0.200000,Y=0.200000)" true :!class /Script/Engine.SplineMeshComponent)
        (else
          (SplineMesh|SetEndScale _returnvalue "(X=0.200000,Y=0.200000)" true :!class /Script/Engine.SplineMeshComponent)
          (SplineMesh|SetStartScale _returnvalue "(X=0.200000,Y=0.200000)" true :!class /Script/Engine.SplineMeshComponent)))
      (Utilities|Array|Add (Variables|Default|GetSplineMeshPool) _returnvalue))
    (elif (< (LocalVariables|GetNewPosNum) (LocalVariables|GetOldPosNum))
      (for _index_2 (range (LocalVariables|GetNewPosNum) (- (LocalVariables|GetOldPosNum) 1))
        (Rendering|SetVisibility (Utilities|Array|Get(acopy) (Variables|Default|GetSplineMeshPool) _index_2) false true)
        (Development|SetHiddeninGame (Utilities|Array|Get(acopy) (Variables|Default|GetSplineMeshPool) _index_2) true true))
      (else
        (return))))
  (return))

(fn SetSplineMesh
  (params (ArrPoints :type Array%20of%20Vectors))
  (for _index (range 0 (- (Utilities|Array|Length ArrPoints) 2))
    (bind _outputpin (CallFunction|GetOneSplineMesh _index))
    (SplineMesh|SetStartandEnd _outputpin (CallFunction|WorldtoRelative (Utilities|Array|Get(acopy) ArrPoints _index)) (- (CallFunction|WorldtoRelative (Utilities|Array|Get(acopy) ArrPoints (+ _index 1))) (CallFunction|WorldtoRelative (Utilities|Array|Get(acopy) ArrPoints _index))) (CallFunction|WorldtoRelative (Utilities|Array|Get(acopy) ArrPoints (+ _index 1))) (- (CallFunction|WorldtoRelative (Utilities|Array|Get(acopy) ArrPoints (+ _index 1))) (CallFunction|WorldtoRelative (Utilities|Array|Get(acopy) ArrPoints _index))) true :!class /Script/Engine.SplineMeshComponent))
  (return))

(fn SetArrowMesh
  (params (ArrPoints :type Array%20of%20Vectors))
  (bind _staticarrowmesh (Variables|Default|GetStaticArrowMesh))
  (if (> (Utilities|Array|Length ArrPoints) 0)
    (bind _output_get (CallFunction|GetArrowMesh (CallFunction|WorldtoRelative (Utilities|Array|Get(acopy) ArrPoints)) (Math|Conversions|RotationFromXVector (- (CallFunction|WorldtoRelative (Utilities|Array|Get(acopy) ArrPoints 1)) (CallFunction|WorldtoRelative (Utilities|Array|Get(acopy) ArrPoints))))))
    (Components|StaticMesh|SetStaticMesh _output_get (Variables|Default|GetArrowMesh))
    (Rendering|SetRenderCustomDepth _output_get false)
    (Rendering|Material|SetMaterial _output_get 0 (Variables|Default|GetM_Arrow))
    (Collision|SetCollisionEnabled _output_get "NoCollision")
    (if (Variables|Default|GetScaleChange)
      (Transformation|SetWorldScale3D _output_get "0.200000,0.200000, 0")
      (Transformation|AddLocalOffset _output_get "-49.799999, 0, 0" false false)
      (else
        (Transformation|SetWorldScale3D _output_get "0.200000,0.200000, 0")
        (Transformation|AddLocalOffset _output_get "-49.799999, 0, 0" false false)))
    (return)
    (else
      (Rendering|SetVisibility _staticarrowmesh false false)
      (Development|SetHiddeninGame _staticarrowmesh true false)
      (return))))

(fn WorldtoRelative
  (params (WorldLocation :type Vector%20%28by%20ref%29))
  (return (Math|Transform|InverseTransformLocation (Transformation|GetActorTransform) WorldLocation)))

(fn GetArrowMesh
  (params (RelativePosition :type Vector%20%28by%20ref%29) (RelativeRotator :type Rotator%20%28by%20ref%29))
  (if (Utilities|IsValid (Variables|Default|GetStaticArrowMesh))
    (Transformation|SetRelativeLocationAndRotation (Variables|Default|GetStaticArrowMesh) RelativePosition RelativeRotator false false)
    (else
      (bind _returnvalue (AddComponent|AddStaticMeshComponent false (Math|Transform|MakeTransform RelativePosition RelativeRotator "1,1,1")))
      (Variables|Default|SetStaticArrowMesh _returnvalue)))
  (Rendering|SetVisibility (Variables|Default|GetStaticArrowMesh) true false)
  (Development|SetHiddeninGame (Variables|Default|GetStaticArrowMesh) false false)
  (return (Variables|Default|GetStaticArrowMesh)))

(fn GetOneSplineMesh
  (params (IndexNum :type Integer%20%28by%20ref%29))
  (LocalVariables|SetSplineMeshItem (Utilities|Array|Get(acopy) (Variables|Default|GetSplineMeshPool) IndexNum))
  (Rendering|SetVisibility (LocalVariables|GetSplineMeshItem) true true)
  (Development|SetHiddeninGame (LocalVariables|GetSplineMeshItem) false true)
  (return (LocalVariables|GetSplineMeshItem)))

(fn Fadein
  (if (<= (Variables|Default|GetOpacity) 1.0)
    (Variables|Default|SetOpacity (Math|Float|Clamp(Float) (+ (Variables|Default|GetOpacity) (* (Utilities|Time|GetWorldDeltaSeconds) 0.4)) 0.0 1.1))
    ;[1 1 1] 这里强行改成1，不渐入，不然要一直调用
    (bind _output_get (Variables|Default|SetOpacity 1.0))
    (Rendering|Material|SetScalarParameterValue (Variables|Default|GetM_Line) "Opacity" _output_get :!class /Script/Engine.MaterialInstanceDynamic)
    (Rendering|Material|SetScalarParameterValue (Variables|Default|GetM_Arrow) "Opacity" _output_get :!class /Script/Engine.MaterialInstanceDynamic)
    (Development|PrintString (Utilities|String|ToString(Float) _output_get))
    (else
      (return))))

(fn FadeOut
  (if (>= (Variables|Default|GetOpacity) 0.0)
    (bind _output_get (Variables|Default|SetOpacity (Math|Float|Clamp(Float) (- (Variables|Default|GetOpacity) (* (Utilities|Time|GetWorldDeltaSeconds) 2.0)) -0.1)))
    (Rendering|Material|SetScalarParameterValue (Variables|Default|GetM_Line) "Opacity" _output_get :!class /Script/Engine.MaterialInstanceDynamic)
    (Rendering|Material|SetScalarParameterValue (Variables|Default|GetM_Arrow) "Opacity" _output_get :!class /Script/Engine.MaterialInstanceDynamic)
    (return true)
    (else
      (return false))))